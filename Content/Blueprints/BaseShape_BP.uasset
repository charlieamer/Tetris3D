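; BaseShape_BP is a base shape actor that animates grid-style moves and 90-degree rotations driven by shape events.
; On initialization it snaps to its world location and binds the move and rotate events.
; Timelines lerp the actor toward the new location or accumulated target rotation, restarting from the current transform on each event.
; When a move animation finishes on a dropped shape, it calls ShapeDone.
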(event `self.ReceiveBeginPlay`
  ;[1 1 1] Animated shape movement
  (add `self.ShapeInitialized` (delegate `OnShapeInitialized`)))

(event `OnShapeInitialized`
  ;[1 1 1] Animated shape movement
  (add `self.ShapeMoved` (delegate `OnShapeMoved`))
  (`self.K2_SetActorLocation` (`self.GetWorldLocation`))
  ;[1 1 1] Animated shape rotation
  (add `self.ShapeRotated` (delegate `OnRotated`)))

(event `OnRotated` :!signature `self.ShapeRotated`
  (params (Axis :type "Vector Structure"))
  ;[1 1 1] Animated shape rotation
  (set `self.EndingRotation` (`KismetMathLibrary.ComposeRotators` (`self.EndingRotation`) (`KismetMathLibrary.RotatorFromAxisAndAngle` Axis 90.0)))
  (set `self.StartingRotation` (`self.K2_GetActorRotation`))
  (bind (_direction _dropdisplacement) (`Timeline|RotateTimeline` :!via `PlayFromStart`)
    (:`Update`
      (`self.K2_SetActorRotation` (`KismetMathLibrary.RLerp` (`self.StartingRotation`) (`self.EndingRotation`) _dropdisplacement true)))))

(event `OnShapeMoved`
  ;[1 1 1] Animated shape movement
  (set `self.StartingPosition` (`self.K2_GetActorLocation`))
  (set `self.EndingPosition` (`self.GetWorldLocation`))
  (bind (_direction _dropdisplacement) (`Timeline|DropTimeline` :!via `PlayFromStart`)
    (:`Update`
      (`self.K2_SetActorLocation` (`KismetMathLibrary.VLerp` (`self.StartingPosition`) (`self.EndingPosition`) _dropdisplacement)))
    (:`Finished`
      (if (`self.bWasDropped`)
        (`self.ShapeDone` self)))))

(fn `UserConstructionScript`)